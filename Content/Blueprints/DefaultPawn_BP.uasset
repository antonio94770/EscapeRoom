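; Default pawn Blueprint that lets the player yaw an object held by its Grabber component.
; Numpad 4 and 6 set the rotation direction while held and reset the yaw value on release.
; While grabbing, Tick steps that value each frame so rotation accelerates, applies it scaled by delta time to the hit actor from the Grabber's reach query, and prints the delta for debugging.
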(event `Key|NumPadSix`
  (params (Key :type "Key Structure"))
  ;[1 1 1] Input Rotation
  (:`Pressed`
    (set `self.ShouldRotate` true)
    (set `self.IsRotatingLeft` false))
  (:`Released`
    (set `self.ShouldRotate` false)
    (set `self.YawValue` 0.0)))

(event `Key|NumPadFour`
  (params (Key :type "Key Structure"))
  ;[1 1 1] Input Rotation
  (:`Pressed`
    (set `self.ShouldRotate` true)
    (set `self.IsRotatingLeft` true))
  (:`Released`
    (set `self.ShouldRotate` false)
    (set `self.YawValue` 0.0)))

(event `self.ReceiveTick`
  (params (DeltaSeconds :type "Float (single-precision)"))
  (bind _yawvalue (`self.YawValue`))
  (bind _grabber (`self.Grabber`))
  (bind _returnvalue (`KismetMathLibrary.MakeRotator` 0.0 0.0 (* _yawvalue DeltaSeconds)))
  ;[1 1 1] Rotation Left/Right
  (if (`Grabber.IsGrabbed` _grabber)
    (if (`self.ShouldRotate`)
      (if (`self.IsRotatingLeft`)
        (`/Engine/EditorBlueprintResources/StandardMacros.DecrementFloat` _yawvalue
          (:`  `
            _))
        (else
          (`/Engine/EditorBlueprintResources/StandardMacros.IncrementFloat` _yawvalue
            (:`  `
              _))))
      (`self.K2_AddActorLocalRotation` (`.HitActor` (`GameplayStatics.BreakHitResult` (`Grabber.GetFirstPhysicsBodyInReach` _grabber))) _returnvalue false false)
      (`KismetSystemLibrary.PrintString` (`KismetStringLibrary.Conv_RotatorToString` _returnvalue)))))

(fn `UserConstructionScript`)